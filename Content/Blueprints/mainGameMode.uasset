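; Game mode that drives escalating enemy waves from the EnemySpawner actors placed in the level.
; On BeginPlay it caches all spawners and, if any exist, spawns a wave immediately and starts a looping timer that repeats it every few seconds.
; Each wave picks one spawner at random, calls its SpawnEnemy in a loop bounded by NumSpawn, then increments NumSpawn so the next wave is larger.
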(event `self.ReceiveBeginPlay`
  (bind _outactors (`GameplayStatics.GetAllActorsOfClass` "/Game/Blueprints/enemySpawner.enemySpawner_C"))
  (if (> (`KismetArrayLibrary.Array_Length` _outactors) 0)
    (set `self.spawnerArray` _outactors)
    (`self.spawnWave`)
    (`KismetSystemLibrary.K2_SetTimer` null "spawnWave" 6.0 true)))

(fn `spawnWave`
  (locals (targetSpawner :type "/Game/Blueprints/enemySpawner Object Reference"))
  (bind _spawnerarray (`self.spawnerArray`))
  (bind _output_get (set `local.targetSpawner` (`|GetArrayItem` _spawnerarray (`KismetMathLibrary.RandomInteger` (`KismetArrayLibrary.Array_Length` _spawnerarray)))))
  (for _ (range (+ (`self.numSpawn`) 1))
    (`/Game/Blueprints/enemySpawner.spawnEnemy` _output_get))
  (`/Engine/EditorBlueprintResources/StandardMacros.IncrementInt` (`self.numSpawn`)))

(fn `UserConstructionScript`)