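; Player character Blueprint for what appears to be a twin-stick shooter, with world-axis movement and mouse or stick aiming.
; On BeginPlay it spawns and attaches a Visor_weapon, whose trigger follows primaryFire, and shows the cursor.
; Each tick turns the capsule's yaw toward the cursor trace hit, while look axes set control rotation past a deadzone.
; Damage updates health, with debug prints for health and death.
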(event `self.ReceiveBeginPlay`
  (`parent.ReceiveBeginPlay`)
  (`|ExecutionSequence`
    (:`then_0`
      (bind _returnvalue (`|SpawnActorFromClass` "/Game/Blueprints/visor_weapon.visor_weapon_C" (`SceneComponent.K2_GetComponentToWorld` (`self.tempWeaponMark`)) "AlwaysSpawn" "OverrideRootScale" null null))
      (bind _output_get (set `self.primaryWeapon` _returnvalue))
      (`self.K2_AttachToComponent` _output_get (`self.tempWeaponMark`) "None" "KeepWorld" "KeepWorld" "KeepWorld" true))
    (:`then_1`
      (set `PlayerController.bShowMouseCursor` true (`GameplayStatics.GetPlayerController` 0)))))

(event `self.ReceiveTick`
  (params (DeltaSeconds :type "Float (single-precision)"))
  (`parent.ReceiveTick` DeltaSeconds)
  (`self.updateMouseAim`))

(event `InputAction|primaryFire`
  (params (Key :type "Key Structure"))
  (bind _primaryweapon (`self.primaryWeapon`))
  (:`Pressed`
    (`/Game/Blueprints/visor_weapon.pressTrigger` _primaryweapon))
  (:`Released`
    (`/Game/Blueprints/visor_weapon.releaseTrigger` _primaryweapon)))

(event `InputAxis|MoveNorth`
  (params (AxisValue :type "Float (single-precision)"))
  ;[1 1 1] Controller movement
  (`self.AddMovementInput` (1.0 0.0 0.0) AxisValue))

(event `InputAxis|MoveEast`
  (params (AxisValue :type "Float (single-precision)"))
  ;[1 1 1] Controller movement
  (`self.AddMovementInput` (0.0 1.0 0.0) AxisValue))

(event `InputAxis|LookNorth`
  (params (AxisValue :type "Float (single-precision)"))
  ;[1 1 1] Controller look rotation
  (bind _returnvalue (`KismetMathLibrary.MakeVector` AxisValue (* -1 (stale `InputAxis|LookEast` AxisValue))))
  (if (> (`KismetMathLibrary.VSize` _returnvalue) 0.25) :!label _label
    (`Controller.SetControlRotation` (`self.GetController`) (`KismetMathLibrary.Conv_VectorToRotator` _returnvalue))))

(event `InputAxis|LookEast`
  (params (AxisValue :type "Float (single-precision)"))
  ;[1 1 1] Controller look rotation
  (goto _label))

(event `self.ReceiveAnyDamage`
  (params (Damage :type "Float (single-precision)") (DamageType :type "DamageType Object Reference") (InstigatedBy :type "Controller Object Reference") (DamageCauser :type "Actor Object Reference"))
  (`self.updateHealth` Damage)
  (`KismetSystemLibrary.PrintString` (`KismetStringLibrary.Conv_DoubleToString` (`self.health`)))
  (if (`self.isDead`)
    (`KismetSystemLibrary.PrintString` "Dead")))

(fn `updateMouseAim`
  (bind (_returnvalue_roll _returnvalue_pitch) (`KismetMathLibrary.BreakRotator` (`self.K2_GetActorRotation`)))
  (bind (_returnvalue_roll_2 _returnvalue_pitch_2 _returnvalue_yaw) (`KismetMathLibrary.BreakRotator` (`KismetMathLibrary.FindLookAtRotation` (`self.K2_GetActorLocation`) (`.Location` (`GameplayStatics.BreakHitResult` (`PlayerController.GetHitResultUnderCursorByChannel` (`GameplayStatics.GetPlayerController` 0) "TraceTypeQuery1" true))))))
  (`SceneComponent.K2_SetWorldRotation` (`self.CapsuleComponent`) (`KismetMathLibrary.MakeRotator` _returnvalue_roll _returnvalue_pitch _returnvalue_yaw) false false))

(fn `UserConstructionScript`
  (`parent.UserConstructionScript`))