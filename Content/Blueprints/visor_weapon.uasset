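; Visor weapon Blueprint that fires projectiles automatically while its trigger is held.
; A trigger press passes a DoOnce, fires at once and starts a looping timer at the RoundsPerSecond rate; release clears the timer and resets the gate.
; Each shot spawns a BasicProjectile at the SpawnArrow transform.
; An unconnected hitscan path that line-traces pawns and damages basicEnemy actors remains in the graph but never runs.
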(event `pressTrigger`
  (`/Engine/EditorBlueprintResources/StandardMacros.DoOnce` false :!label _label
    (:`Completed`
      (`self.fire`)
      (`KismetSystemLibrary.K2_SetTimer` null "fire" (/ 1.0 (`self.roundsPerSecond`)) true))))

(event `releaseTrigger`
  (`KismetSystemLibrary.K2_ClearTimer` null "fire")
  (goto _label :!via `Reset`))

(event `fire`
  (`|SpawnActorFromClass` "/Game/Blueprints/basicProjectile.basicProjectile_C" (`SceneComponent.K2_GetComponentToWorld` (`self.spawnArrow`)) "Undefined" "OverrideRootScale" null null))

(fn `UserConstructionScript`)