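; Basic enemy actor that damages the player on contact and dies from a single hit.
; On overlap with a playerCharacter it applies a heavy fixed amount of damage, and any damage it receives destroys it immediately, with no health tracking.
; The construction script creates dynamic material instances on the first two mesh material slots and tints their body color dark grey.
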(event `self.ReceiveActorBeginOverlap`
  (params (OtherActor :type "Actor Object Reference"))
  (`parent.ReceiveActorBeginOverlap` OtherActor)
  (bind _asplayer_character (cast `/Game/Blueprints/playerCharacter` OtherActor))
  (`GameplayStatics.ApplyDamage` _asplayer_character 100.0))

(event `self.ReceiveAnyDamage`
  (params (Damage :type "Float (single-precision)") (DamageType :type "DamageType Object Reference") (InstigatedBy :type "Controller Object Reference") (DamageCauser :type "Actor Object Reference"))
  (`self.K2_DestroyActor`))

(fn `UserConstructionScript`
  (`parent.UserConstructionScript`)
  (bind _returnvalue (`PrimitiveComponent.CreateDynamicMaterialInstance` (`self.Mesh`) 0 null))
  (`MaterialInstanceDynamic.SetVectorParameterValue` _returnvalue "bodyColor" (struct :`R` 0.119792 :`G` 0.119792 :`B` 0.119792 :`A` 1.0))
  (bind _returnvalue_2 (`PrimitiveComponent.CreateDynamicMaterialInstance` (`self.Mesh`) 1 null))
  (`MaterialInstanceDynamic.SetVectorParameterValue` _returnvalue_2 "bodyColor" (struct :`R` 0.119792 :`G` 0.119792 :`B` 0.119792 :`A` 1.0)))